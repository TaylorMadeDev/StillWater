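; Player character Blueprint for a flipbook-animated sprite with four-directional movement through Enhanced Input.
; BeginPlay adds the player mapping context, and IA_Move drives movement input along the actor's forward and right vectors.
; Exact axis values select walk flipbooks and record LastFacing, with left and right sharing a side flipbook flipped by rotating the sprite.
; Releasing the input prints LastFacing and sets the matching idle flipbook.
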(event `self.ReceiveBeginPlay`
  (`EnhancedInputSubsystemInterface.AddMappingContext` (pcsubsystem `EnhancedInputLocalPlayerSubsystem` (`GameplayStatics.GetPlayerController` 0)) "/Game/Movement/IMC_Player.IMC_Player" 0 (struct)))

(event `EnhancedInput|/Game/Movement/IA_Move`
  (params (ActionValue :type "Vector2D Structure") (ElapsedSeconds :type "Float (double-precision)") (TriggeredSeconds :type "Float (double-precision)") (InputAction :type "InputAction Object Reference" :default "/Game/Movement/IA_Move.IA_Move"))
  (bind (_x _y) (`KismetMathLibrary.BreakVector2D` ActionValue))
  (bind _sprite (`self.Sprite`))
  (bind _sprite_2 (`self.Sprite`))
  (:`Triggered`
    (if (== _x -1.0)
      (`PaperFlipbookComponent.SetFlipbook` _sprite_2 "/Game/Animation/FB_Walk_SideWays.FB_Walk_SideWays")
      (`SceneComponent.K2_SetRelativeRotation` _sprite_2 (struct :`Yaw` 180.0) false false)
      (set `self.LastFacing` "NewEnumerator2")
      (elif (== _x 1.0)
        (`PaperFlipbookComponent.SetFlipbook` _sprite_2 "/Game/Animation/FB_Walk_SideWays.FB_Walk_SideWays")
        (`SceneComponent.K2_SetRelativeRotation` :`self` _sprite_2)
        (set `self.LastFacing` "NewEnumerator3")
        (elif (== _y -1.0)
          (`PaperFlipbookComponent.SetFlipbook` _sprite "/Game/Animation/FB_Walk_Up.FB_Walk_Up")
          (set `self.LastFacing` "NewEnumerator0")
          (elif (== _y 1.0)
            (`PaperFlipbookComponent.SetFlipbook` _sprite "/Game/Animation/FB_Walk_Down.FB_Walk_Down")
            (set `self.LastFacing` "NewEnumerator1")))))))

(event `EnhancedInput|/Game/Movement/IA_Move`
  (params (ActionValue :type "Vector2D Structure") (ElapsedSeconds :type "Float (double-precision)") (TriggeredSeconds :type "Float (double-precision)") (InputAction :type "InputAction Object Reference" :default "/Game/Movement/IA_Move.IA_Move"))
  (bind (_x _y) (`KismetMathLibrary.BreakVector2D` ActionValue))
  (:`Triggered`
    (`self.AddMovementInput` (`self.GetActorRightVector`) _y)
    (`self.AddMovementInput` (`self.GetActorForwardVector`) _x)))

(event `EnhancedInput|/Game/Movement/IA_Move`
  (params (ActionValue :type "Vector2D Structure") (ElapsedSeconds :type "Float (double-precision)") (TriggeredSeconds :type "Float (double-precision)") (InputAction :type "InputAction Object Reference" :default "/Game/Movement/IA_Move.IA_Move"))
  (bind _lastfacing (`self.LastFacing`))
  (bind _sprite (`self.Sprite`))
  (:`Completed`
    (`KismetSystemLibrary.PrintString` (`|GetEnumeratorNameAsString` _lastfacing))
    (switch `/Game/E_FacingDirection` _lastfacing
      (:`NewEnumerator0`
        (`PaperFlipbookComponent.SetFlipbook` _sprite "/Game/Animation/FB_Idle_Back.FB_Idle_Back"))
      (:`NewEnumerator1`
        (`PaperFlipbookComponent.SetFlipbook` _sprite "/Game/Animation/FB_Idle_Front.FB_Idle_Front"))
      (:`NewEnumerator2`
        (`SceneComponent.K2_SetRelativeRotation` _sprite (struct :`Yaw` 180.0) false false)
        (`PaperFlipbookComponent.SetFlipbook` _sprite "/Game/Animation/FB_Idle_Side.FB_Idle_Side"))
      (:`NewEnumerator3`
        (`SceneComponent.K2_SetRelativeRotation` :`self` _sprite)
        (`PaperFlipbookComponent.SetFlipbook` _sprite "/Game/Animation/FB_Idle_Side.FB_Idle_Side")))))

(fn `UserConstructionScript`)